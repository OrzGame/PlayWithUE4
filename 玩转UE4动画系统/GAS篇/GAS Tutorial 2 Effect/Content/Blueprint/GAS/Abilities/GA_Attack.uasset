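; Gameplay ability for a melee attack that plays the attack montage on the avatar's skeletal mesh.
; On the montage's "Hit" notify, it runs a short-range target trace with debug drawing and applies GE_Hit to a detected target that has an Ability System Component.
; The ability ends when the montage completes, with no handling for interruption, and stops the montage on end.
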(event `self.K2_ActivateAbility`
  (bind (_returnvalue_owneractor _returnvalue_avataractor _returnvalue_playercontroller _returnvalue_abilitysystemcomponent) (break `GameplayAbilityActorInfo` (`self.GetActorInfo`)))
  (bind (_returnvalue_owneractor_2 _returnvalue_avataractor_2 _returnvalue_playercontroller_2 _returnvalue_abilitysystemcomponent_2 _returnvalue_skeletalmeshcomponent) (break `GameplayAbilityActorInfo` (`self.GetActorInfo`)))
  (bind (_returnvalue_owneractor_3 _returnvalue_avataractor_3) (break `GameplayAbilityActorInfo` (`self.GetActorInfo`)))
  (bind _notifyname (`|PlayMontage` _returnvalue_skeletalmeshcomponent "/Game/Mannequin/Animations/PunchPack/Attack_Montage.Attack_Montage")
    (:`OnCompleted`
      (`self.K2_EndAbility`))
    (:`OnNotifyBegin`
      (if (== _notifyname "Hit")
        (bind (_detected _target) (`TraceFunctions.TraceForTarget` _returnvalue_avataractor_3 100.0 "ForDuration"))
        (if _detected
          (bind _returnvalue (`AbilitySystemBlueprintLibrary.GetAbilitySystemComponent` _target))
          (`/Engine/EditorBlueprintResources/StandardMacros.IsValid` _returnvalue
            (:`Is Valid`
              (`AbilitySystemComponent.BP_ApplyGameplayEffectToTarget` :`self` _returnvalue_abilitysystemcomponent :`GameplayEffectClass` "/Game/Blueprint/GAS/Effects/GE_Hit.GE_Hit_C" :`Target` _returnvalue))))))))

(event `self.K2_OnEndAbility`
  (params (bWasCancelled :type Boolean))
  (`self.MontageStop` -1.0))