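; BP_PlayerCharacter is the player character Blueprint, turning input into movement and ability requests.
; The MoveRight axis adds movement along the world negative Y axis, giving side-scroller style motion.
; Jump and Attack presses go through the Gameplay Ability System, activating abilities by the Ability.Jump and Ability.Attack tags instead of running that logic directly.
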(event `InputAxis|MoveRight`
  (params (AxisValue :type "Float (single-precision)"))
  (`self.AddMovementInput` (0.0 -1.0 0.0) AxisValue))

(event `InputAction|Jump`
  (params (Key :type "Key Structure"))
  (:`Pressed`
    (`AbilitySystemComponent.TryActivateAbilitiesByTag` (`self.AbilitySystemComponent`) (`BlueprintGameplayTagLibrary.MakeGameplayTagContainerFromTag` (struct :`TagName` "Ability.Jump")) true)))

(event `InputAction|Attack`
  (params (Key :type "Key Structure"))
  (:`Pressed`
    (`AbilitySystemComponent.TryActivateAbilitiesByTag` (`self.AbilitySystemComponent`) (`BlueprintGameplayTagLibrary.MakeGameplayTagContainerFromTag` (struct :`TagName` "Ability.Attack")) true)))

(fn `UserConstructionScript`
  (`parent.UserConstructionScript`))