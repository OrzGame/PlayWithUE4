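; GA_OnHit is a Gameplay Ability that briefly flags a character as punched for its animation Blueprint.
; On activation it requires an RPGCharacterBase owner, sets Punched on the mesh's ThirdPerson_AnimBP, then ends itself after a short fixed delay.
; OnEndAbility repeats the owner and anim instance casts and clears the flag.
; A failed cast on activation stops the graph before EndAbility is reached.
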(event `self.K2_ActivateAbility`
  (bind (_returnvalue_owneractor _returnvalue_avataractor _returnvalue_playercontroller _returnvalue_abilitysystemcomponent _returnvalue_skeletalmeshcomponent) (break `GameplayAbilityActorInfo` (`self.GetActorInfo`)))
  (cast `RPGCharacterBase` _returnvalue_owneractor)
  (bind _asthird_person_anim_bp (cast `/Game/Mannequin/Animations/ThirdPerson_AnimBP` (`SkeletalMeshComponent.GetAnimInstance` _returnvalue_skeletalmeshcomponent)))
  (set `/Game/Mannequin/Animations/ThirdPerson_AnimBP.Punched` true _asthird_person_anim_bp)
  (`KismetSystemLibrary.Delay` 0.2)
  (`self.K2_EndAbility`))

(event `self.K2_OnEndAbility`
  (params (bWasCancelled :type Boolean))
  (bind (_returnvalue_owneractor _returnvalue_avataractor _returnvalue_playercontroller _returnvalue_abilitysystemcomponent _returnvalue_skeletalmeshcomponent) (break `GameplayAbilityActorInfo` (`self.GetActorInfo`)))
  (cast `RPGCharacterBase` _returnvalue_owneractor)
  (bind _asthird_person_anim_bp (cast `/Game/Mannequin/Animations/ThirdPerson_AnimBP` (`SkeletalMeshComponent.GetAnimInstance` _returnvalue_skeletalmeshcomponent)))
  (set `/Game/Mannequin/Animations/ThirdPerson_AnimBP.Punched` false _asthird_person_anim_bp))