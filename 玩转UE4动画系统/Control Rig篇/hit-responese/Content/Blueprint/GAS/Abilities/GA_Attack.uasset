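; GA_Attack is a Gameplay Ability for a melee punch that plays an attack montage and ends when it completes.
; On the "Hit" notify, it runs a short trace from the right upper-arm socket, with debug drawing enabled.
; A detected target with an Ability System Component receives GE_Hit, and its AnimBP gets the hit normal as PunchDirection.
; Ending the ability stops the montage.
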(event `self.K2_ActivateAbility`
  (bind (_returnvalue_owneractor _returnvalue_avataractor _returnvalue_playercontroller _returnvalue_abilitysystemcomponent) (break `GameplayAbilityActorInfo` (`self.GetActorInfo`)))
  (bind (_returnvalue_owneractor_2 _returnvalue_avataractor_2 _returnvalue_playercontroller_2 _returnvalue_abilitysystemcomponent_2 _returnvalue_skeletalmeshcomponent) (break `GameplayAbilityActorInfo` (`self.GetActorInfo`)))
  (bind (_returnvalue_owneractor_3 _returnvalue_avataractor_3 _returnvalue_playercontroller_3 _returnvalue_abilitysystemcomponent_3 _returnvalue_skeletalmeshcomponent_2) (break `GameplayAbilityActorInfo` (`self.GetActorInfo`)))
  (bind _notifyname (`|PlayMontage` _returnvalue_skeletalmeshcomponent "/Game/Mannequin/Animations/PunchPack/Attack_Montage.Attack_Montage")
    (:`OnCompleted`
      (`self.K2_EndAbility`))
    (:`OnNotifyBegin`
      (if (== _notifyname "Hit")
        (bind (_detected _target _result) (`TraceFunctions.TraceForTarget` _returnvalue_avataractor_3 (`SceneComponent.GetSocketLocation` _returnvalue_skeletalmeshcomponent_2 "upperarm_r") 60.0 "ForDuration"))
        (if _detected
          (bind _returnvalue (`AbilitySystemBlueprintLibrary.GetAbilitySystemComponent` _target))
          (`/Engine/EditorBlueprintResources/StandardMacros.IsValid` _returnvalue
            (:`Is Valid`
              (`AbilitySystemComponent.BP_ApplyGameplayEffectToTarget` :`self` _returnvalue_abilitysystemcomponent :`GameplayEffectClass` "/Game/Blueprint/GAS/Effects/GE_Hit.GE_Hit_C" :`Target` _returnvalue)
              (bind _asthird_person_anim_bp (cast `/Game/Mannequin/Animations/ThirdPerson_AnimBP` (`SkeletalMeshComponent.GetAnimInstance` (`Character.Mesh` _target))))
              (set `/Game/Mannequin/Animations/ThirdPerson_AnimBP.PunchDirection` (`.Normal` (`GameplayStatics.BreakHitResult` _result)) _asthird_person_anim_bp))))))))

(event `self.K2_OnEndAbility`
  (params (bWasCancelled :type Boolean))
  (`self.MontageStop` -1.0))